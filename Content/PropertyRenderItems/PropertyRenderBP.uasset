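; PropertyRenderBP is a world-space text label that displays a wolf's age, gender and rank.
; Events store those properties and set the owner wolf.
; Each Tick, once IsAttached is set, it rotates the actor along the camera-to-text direction and rebuilds the three-line prefixed string.
; SetIsAttached runs validity and NPCWolfBP cast checks, but every visible branch sets the flag true.
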(event `SetWolfProperties`
  (params (wolfRank :type String) (wolfAge :type String) (wolfGender :type String))
  (set `self.WolfRank` wolfRank)
  (set `self.WolfAge` wolfAge)
  (set `self.WolfGender` wolfGender))

(event `BPSetWolfOWner`
  (params (ownerWolfToSet :type "/Game/Wolves/NPCWolfBP Object Reference"))
  (`self.SetOwnerWolf` ownerWolfToSet))

(event `self.ReceiveTick`
  (params (DeltaSeconds :type "Float (single-precision)"))
  (if (`self.IsAttached`)
    (`self.Rotate Property Render To Player` :!label _label)
    (`self.ComposeAndSetPropertyText`)
    (else
      (`self.SetIsAttached`)
      (if (`self.IsAttached`)
        (goto _label)))))

(fn `ComposeAndSetPropertyText`
  (set `self.FinalString` (`KismetStringLibrary.Concat_StrStr` (`KismetStringLibrary.Concat_StrStr` (`KismetStringLibrary.Concat_StrStr` (`KismetStringLibrary.Concat_StrStr` (`KismetStringLibrary.Concat_StrStr` (`self.AgePrefix`) (`self.WolfAge`)) "<br>") (`KismetStringLibrary.Concat_StrStr` (`self.GenderPrefix`) (`self.WolfGender`))) "<br>") (`KismetStringLibrary.Concat_StrStr` (`self.RankPrefix`) (`self.WolfRank`))))
  (`TextRenderComponent.SetText` (`self.PropertyRender`) (`self.FinalString`)))

(fn `Rotate Property Render To Player`
  (`self.SetActorRotation` (`KismetMathLibrary.MakeRotFromX` (- (`SceneComponent.K2_GetComponentLocation` (`self.PropertyRender`)) (`self.K2_GetActorLocation` (`GameplayStatics.GetPlayerCameraManager` 0))))))

(fn `SetIsAttached`
  (`/Engine/EditorBlueprintResources/StandardMacros.IsValid` null
    (:`Is Valid`
      (set `self.IsAttached` true :!label _label))
    (:`Is Not Valid`
      (bind _asnpcwolf_bp (cast `/Game/Wolves/NPCWolfBP` null)
        (:`then`
          (`/Engine/EditorBlueprintResources/StandardMacros.IsValid` _asnpcwolf_bp
            (:`Is Valid`
              (goto _label))
            (:`Is Not Valid`
              _)))
        (:`CastFailed`
          _))
      (set `self.IsAttached` true))))

(fn `UserConstructionScript`)