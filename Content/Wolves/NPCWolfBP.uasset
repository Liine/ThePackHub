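; NPC wolf character Blueprint that shows its pack rank, age and gender on an attached property text render.
; When the render spawns successfully, it casts it to PropertyRenderBP, registers itself as owner and caches the WolfGame game mode.
; Each Tick, while the render is valid, it pushes pack manager property strings to it and sets walk speed from speed rate times speed value.
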(event `self.OnPropertyRenderSpawned`
  (params (success :type Boolean))
  ;[1 1 1] Fetch Property Render and WolfGame
  (if success
    (bind _asproperty_render_bp (cast `/Game/PropertyRenderItems/PropertyRenderBP` (`self.mPropertyTextRender`)))
    (set `self.BP_PropertyRender` _asproperty_render_bp)
    (`/Game/PropertyRenderItems/PropertyRenderBP.BPSetWolfOWner` (`self.BP_PropertyRender`) self)
    (bind _aswolf_game (cast `WolfGame` (`GameplayStatics.GetGameMode`)))
    (set `self.mWolfGame` _aswolf_game)))

(event `self.ReceiveTick`
  (params (DeltaSeconds :type "Float (single-precision)"))
  (bind _mpackmemberdata (`self.mPackMemberData`))
  (bind _bp_propertyrender (`self.BP_PropertyRender`))
  (bind _mpackmanager (`WolfGame.mPackManager` (`self.mWolfGame`)))
  ;[1 1 1] Update property render wolf stats
  (`/Engine/EditorBlueprintResources/StandardMacros.IsValid` _bp_propertyrender
    (:`Is Valid`
      (bind _returnvalue (`PackManager.GetPackMemberPropertyString` _mpackmanager _mpackmemberdata "EPP_Rank"))
      (bind _returnvalue_2 (`PackManager.GetPackMemberPropertyString` _mpackmanager _mpackmemberdata "EPP_Age"))
      (bind _returnvalue_3 (`PackManager.GetPackMemberPropertyString` _mpackmanager _mpackmemberdata "EPP_Gender"))
      (`/Game/PropertyRenderItems/PropertyRenderBP.SetWolfProperties` _bp_propertyrender _returnvalue _returnvalue_2 _returnvalue_3)
      (set `CharacterMovementComponent.MaxWalkSpeed` (* (`self.mSpeedRate`) (`self.mSpeedValue`)) (`self.CharacterMovement`)))))

(fn `UserConstructionScript`)